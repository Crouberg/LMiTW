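; BP_Node is a node actor that holds references to connected doors, exposed through GetDoors, and an Id.
; On BeginPlay it warns about empty door references, removes them during iteration and clears its init-success flag.
; It then runs debug-drawn line traces to each door, showing the links for a minute.
; The construction script labels its TextRender with the object name up to the first "e" plus the Id.
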(event `self.ReceiveBeginPlay`
  (bind _bpdoors (`self.BPDoors`))
  (`|ExecutionSequence`
    (:`then_0`
      (for (_array_element _array_index) _bpdoors
        (if (== _array_element null)
          (`KismetSystemLibrary.PrintString` (`KismetStringLibrary.Concat_StrStr` (`KismetSystemLibrary.GetDisplayName` self) ": " "WARNING. Variable DoorRefs have free values") true true (struct :`R` 1.0 :`G` 0.464241 :`A` 1.0) 10.0)
          (`KismetArrayLibrary.Array_Remove` _bpdoors _array_index)
          (set `self.BPsuccessInit?` false))))
    (:`then_1`
      (for _ (`self.BPDoors`)
        _))
    (:`then_2`
      (for _array_element_2 (`self.BPDoors`)
        (`KismetSystemLibrary.LineTraceSingle` :`Start` (`self.K2_GetActorLocation` self) :`End` (`self.K2_GetActorLocation` _array_element_2) :`TraceChannel` "TraceTypeQuery1" :`DrawDebugType` "ForDuration" :`TraceColor` (struct :`R` 0.057249 :`G` 1.0 :`A` 1.0) :`DrawTime` 60.0)))))

(fn `getDoors`
  (returns (DoorOut :type "Array of /Game/LMiTW/Blueprints/GameplayActors/Door/BP_DoorSlider Object Reference"))
  (return (`self.BPDoors`)))

(fn `SetNewIndexInName`
  (params (newIndex :type Integer))
  (bind _returnvalue (`KismetSystemLibrary.GetObjectName` self))
  (`TextRenderComponent.K2_SetText` (`self.TextRender`) (`KismetTextLibrary.Conv_StringToText` (`KismetStringLibrary.Concat_StrStr` (`KismetStringLibrary.GetSubstring` _returnvalue 0 (+ (`KismetArrayLibrary.Array_Find` (`KismetStringLibrary.GetCharacterArrayFromString` _returnvalue) "e") 1)) (`KismetStringLibrary.Conv_IntToString` newIndex)))))

(fn `UserConstructionScript`
  (`self.SetNewIndexInName` (`self.id`)))