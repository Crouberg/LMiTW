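; BP_Optimization applies rendering and performance settings through console commands when play begins.
; A Sequence chain optionally switches to unlit view, then builds commands for screen percentage, view distance, post-process AA, frame cap and scalability quality groups.
; Only the unlit toggle and screen percentage come from variables; other values are hardcoded.
; Values are appended to command names without a separating space, and the GameUserSettings resolution-scale nodes never run.
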(event `self.ReceiveBeginPlay`
  (`|ExecutionSequence`
    (:`then_0`
      (if (`self.UnlitMode?`)
        (`KismetSystemLibrary.ExecuteConsoleCommand` "viewmode unlit" null)))
    (:`then_1`
      ;[1 1 1] 0 to 100
      (`KismetSystemLibrary.ExecuteConsoleCommand` (`KismetStringLibrary.Concat_StrStr` "r.ScreenPercentage " (`KismetStringLibrary.Conv_DoubleToString` (`self.ScreenPercentage`))) null))
    (:`then_2`
      ;[1 1 1] 0 to 1
      (`KismetSystemLibrary.ExecuteConsoleCommand` (`KismetStringLibrary.Concat_StrStr` "r.ViewDistanceScale " (`KismetStringLibrary.Conv_DoubleToString` 0.1)) null))
    (:`then_3`
      (`|ExecutionSequence`
        (:`then_0`
          ;[1 1 1] View distace scale: 0 to 1
          (`KismetSystemLibrary.ExecuteConsoleCommand` (`KismetStringLibrary.Concat_StrStr` "r.ViewDistanceScale " (`KismetStringLibrary.Conv_DoubleToString` 0.1)) null))
        (:`then_1`
          ;[1 1 1] PostProcess Anti-aliasing: 0 to 1
          (`KismetSystemLibrary.ExecuteConsoleCommand` (`KismetStringLibrary.Concat_StrStr` "r.PostProcessAAQuality " (`KismetStringLibrary.Conv_DoubleToString` 0.0)) null))
        (:`then_2`
          ;[1 1 1] Max fps
          (`KismetSystemLibrary.ExecuteConsoleCommand` (`KismetStringLibrary.Concat_StrStr` "t.MaxFPS " (`KismetStringLibrary.Conv_DoubleToString` 100.0)) null))
        (:`then_3`
          (`|ExecutionSequence`
            (:`then_0`
              ;[1 1 1] Motion blur quality 0 3
              (`KismetSystemLibrary.ExecuteConsoleCommand` (`KismetStringLibrary.Concat_StrStr` "sg.PostProcessQuality " (`KismetStringLibrary.Conv_DoubleToString` 3.0)) null))
            (:`then_1`
              ;[1 1 1] Shadow quality 0 3
              (`KismetSystemLibrary.ExecuteConsoleCommand` (`KismetStringLibrary.Concat_StrStr` "sg.ShadowQuality " (`KismetStringLibrary.Conv_DoubleToString` 3.0)) null))
            (:`then_2`
              ;[1 1 1] Texture quality 0 3
              (`KismetSystemLibrary.ExecuteConsoleCommand` (`KismetStringLibrary.Concat_StrStr` "sg.TextureQuality " (`KismetStringLibrary.Conv_DoubleToString` 3.0)) null))
            (:`then_3`
              ;[1 1 1] Texture quality 0 3
              (`KismetSystemLibrary.ExecuteConsoleCommand` (`KismetStringLibrary.Concat_StrStr` "sg.EffectsQuality " (`KismetStringLibrary.Conv_DoubleToString` 3.0)) null))))))))

(fn `UserConstructionScript`)