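; Player character Blueprint with switchable first and third person cameras, PDA toggle and interaction.
; Input events set crouch, run and antigravity flags, which Move Forward passes to the movement component; its axis value feeds both forward and right, as Move Right is empty.
; Getter functions supply animation, movement, footstep audio and PDA access data to other systems.
; Number keys switch PDA access level for testing; crawl is unbound and CanMove always returns true.
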(event `self.ReceiveBeginPlay`
  ;[1 1 1] BeginPlay
  ;[1 1 1] SetDefaultCamera
  (`ActorComponent.SetActive` (`self.CameraFirstPerson`) true false)
  (`ActorComponent.SetActive` (`self.CameraThirdPerson`) false false))

(event `Key|V`
  (params (Key :type "Key Structure"))
  ;[1 1 1] Swtich view camera
  (:`Pressed`
    (`/Engine/EditorBlueprintResources/StandardMacros.FlipFlop`
      (:`A`
        (`ActorComponent.SetActive` (`self.CameraThirdPerson`) true false)
        (`ActorComponent.SetActive` (`self.CameraFirstPerson`) false false))
      (:`B`
        (`ActorComponent.SetActive` (`self.CameraFirstPerson`) true false)
        (`ActorComponent.SetActive` (`self.CameraThirdPerson`) false false)))))

(event `Key|F`
  (params (Key :type "Key Structure"))
  ;[1 1 1] Заглушки
  (:`Pressed`
    (`/Game/LMiTW/Blueprints/Components/BP_PlayerInteractionComponent.Interact` (`self.BP_PlayerInteractionComponent`))))

(event `Key|I`
  (params (Key :type "Key Structure"))
  ;[1 1 1] Заглушки
  (:`Pressed`
    (bind _isa (`/Engine/EditorBlueprintResources/StandardMacros.FlipFlop`)
      (:`A`
        _)
      (:`B`
        _))
    (`SceneComponent.SetVisibility` (`self.BP_PlayerPDA`) _isa true)
    (message `/Game/LMiTW/Blueprints/Interface/BPI_PlayerController.SetPlayerInputMode` (`self.GetController`) (select `bool` _isa :`false` "NewEnumerator2" :`true` "NewEnumerator1" :!type "/Game/LMiTW/Blueprints/Enums/E_InputMode Enum"))))

(event `InputAxis|Move Forward`
  (params (AxisValue :type "Float (single-precision)"))
  ;[1 1 1] Movement
  (message `/Game/LMiTW/Blueprints/Interface/BPI_Movement.PlayerInput` (`self.BP_PlayerControlMovementComponent`) AxisValue (stale `InputAxis|Move Right` AxisValue) (`self.PressKeyCrouch?`) (`self.PressKeyRun?`) (`self.PressKeyCrowl?`) (`self.PressKeyAntiGravityMode?`) false (not (`self.CanMove`))))

(event `InputAxis|Move Right`
  (params (AxisValue :type "Float (single-precision)"))
  ;[1 1 1] Movement
)

(event `InputAxis|Turn`
  (params (AxisValue :type "Float (single-precision)"))
  ;[1 1 1] Mouse
  (bind _output_get (set `self.YawDirection` AxisValue))
  (`self.AddControllerYawInput` _output_get))

(event `InputAxis|LookUp`
  (params (AxisValue :type "Float (single-precision)"))
  ;[1 1 1] Mouse
  (bind _output_get (set `self.PitchDirection` AxisValue))
  (`self.AddControllerPitchInput` _output_get))

(event `Key|LeftControl`
  (params (Key :type "Key Structure"))
  ;[1 1 1] crouch
  (:`Pressed`
    (set `self.PressKeyCrouch?` true :!label _label))
  (:`Released`
    (set `self.PressKeyCrouch?` false :!label _label_2)))

(event `Key|K`
  (params (Key :type "Key Structure"))
  ;[1 1 1] antigravityMode
  (:`Pressed`
    (set `self.PressKeyAntiGravityMode?` true))
  (:`Released`
    (set `self.PressKeyAntiGravityMode?` false)))

(event `Key|C`
  (params (Key :type "Key Structure"))
  ;[1 1 1] crouch
  (:`Pressed`
    (goto _label))
  (:`Released`
    (goto _label_2)))

(event `Key|I`
  (params (Key :type "Key Structure"))
  ;[1 1 1] PDA
  (:`Pressed`
    (`/Engine/EditorBlueprintResources/StandardMacros.FlipFlop`
      (:`A`
        (set `self.PressKeyUsePDA?` true))
      (:`B`
        (set `self.PressKeyUsePDA?` false)))))

(event `Key|LeftShift`
  (params (Key :type "Key Structure"))
  ;[1 1 1] run
  (:`Pressed`
    (set `self.PressKeyRun?` true))
  (:`Released`
    (set `self.PressKeyRun?` false)))

(event `Key|Z`
  (params (Key :type "Key Structure"))
  ;[1 1 1] crowl
)

(event `Key|One`
  (params (Key :type "Key Structure"))
  (:`Pressed`
    (`self.SetPdaAccessLevel` "NewEnumerator0")
    (`KismetSystemLibrary.PrintString` (`KismetStringLibrary.Concat_StrStr` "New Acces Level: " (`|GetEnumeratorNameAsString` (`self.PDA AccessLevel`))) true true (struct :`R` 0.187504 :`G` 1.0 :`A` 1.0) :!label _label)))

(event `Key|Two`
  (params (Key :type "Key Structure"))
  (:`Pressed`
    (`self.SetPdaAccessLevel` "NewEnumerator1")
    (goto _label)))

(event `Key|Three`
  (params (Key :type "Key Structure"))
  (:`Pressed`
    (`self.SetPdaAccessLevel` "NewEnumerator2")
    (goto _label)))

(event `Key|Four`
  (params (Key :type "Key Structure"))
  (:`Pressed`
    (`self.SetPdaAccessLevel` "NewEnumerator3")
    (goto _label)))

(fn `CanMove`
  (returns (Result :type Boolean))
  (return true))

(fn `GetAccessLevel`
  (returns (`Access level` :type "/Game/LMiTW/Blueprints/Enums/E_AcessLevels Enum"))
  (return (`self.GetPdaAccessLevel`)))

(fn `GetPdaAccessLevel`
  (returns (AccessLevel :type "/Game/LMiTW/Blueprints/Enums/E_DoorAccessLevel Enum"))
  (return (`self.PDA AccessLevel`)))

(fn `GetSoundStepInfo`
  (returns (Success :type Boolean) (FootStepsAudioComponent :type "AudioComponent Object Reference") (`FootStepsPlay?` :type Boolean) (`EquipmentPlay?` :type Boolean) (FootStepsVolume :type "Float (double-precision)") (EquipmentVolume :type "Float (double-precision)") (`IsMale?` :type Boolean))
  (return true (`self.FootSteps`) true true 1.0 1.0 true))

(fn `InitializeAnimationParametrs`
  (returns (LMBase_Chracter :type "LMBaseCharacter Object Reference") (BP_ControlMovementComponent :type "/Game/LMiTW/Blueprints/Components/BP_PlayerControlMovementComponent Object Reference"))
  (return self (`self.BP_PlayerControlMovementComponent`)))

(fn `InitializeMovementParametrs`
  (returns (InitParametrs :type "/Game/LMiTW/Blueprints/Structures/S_MovementInitInfo Structure"))
  (return (`self.sMovementAndStamina`)))

(fn `SetPdaAccessLevel`
  (params (NewLevel :type "/Game/LMiTW/Blueprints/Enums/E_DoorAccessLevel Enum" :default "NewEnumerator0"))
  (set `self.PDA AccessLevel` NewLevel))

(fn `UserConstructionScript`)