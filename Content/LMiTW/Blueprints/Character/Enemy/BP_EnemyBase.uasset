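; BP_EnemyBase is the base enemy character, holding AI tuning values and current mode.
; Mode changes set walk speed through a Select over patrol, inspect and combat speeds, dropping to zero on death.
; Getters expose start mode, stage, senses setup, inspecting radius and acceptable distance to the player.
; ProcessAttack is a stub that simply returns true, with no attack logic here.
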(fn `GetAcceptableDistance`
  (returns (Distance :type "Float (double-precision)"))
  (return (`self.AcceptableDistanceToPlayer`)))

(fn `GetInspectingRadius`
  (returns (Radius :type "Float (double-precision)"))
  (return (`self.GetMaxInspectingRadius`)))

(fn `GetMaxInspectingRadius`
  (returns (Radius :type "Float (double-precision)"))
  (return (`self.InspectingMaxRadius`)))

(fn `GetStartMode`
  (returns (Mode :type "/Game/LMiTW/Blueprints/Enums/E_AIMode Enum"))
  (return (`self.StartAIMode`)))

(fn `GetStartSensesSetup`
  (returns (Setup :type "/Game/LMiTW/Blueprints/Structures/S_AISensesSetup Structure"))
  (return (`self.StartSensesSetup`)))

(fn `GetStartStage`
  (returns (Stage :type "/Game/LMiTW/Blueprints/Enums/E_AIStages Enum"))
  (return (`self.StartAIStage`)))

(fn `ProcessAttack`
  (returns (Success :type Boolean))
  (return true))

(fn `SetCurrentMode`
  (params (Mode :type "/Game/LMiTW/Blueprints/Enums/E_AIMode Enum" :default "NewEnumerator0"))
  (set `self.CurrentAIMode` Mode)
  (`self.UpdateMovementSpeedByMode`))

(fn `SetMode`
  (params (NewMode :type "/Game/LMiTW/Blueprints/Enums/E_AIMode Enum" :default "NewEnumerator0"))
  (returns (Success :type Boolean))
  (`self.SetCurrentMode` NewMode)
  (return true))

(fn `UpdateMovementSpeedByMode`
  (bind _inspectspeed (`self.InspectSpeed`))
  (bind _patrolspeed (`self.PatrolSpeed`))
  (set `CharacterMovementComponent.MaxWalkSpeed` (select `/Game/LMiTW/Blueprints/Enums/E_AIMode` (`self.CurrentAIMode`) :`NewEnumerator0` _patrolspeed :`NewEnumerator1` _patrolspeed :`NewEnumerator2` (`self.CombatSpeed`) :`NewEnumerator3` (`self.PatrolSpeed`) :`NewEnumerator5` _inspectspeed :`NewEnumerator6` _inspectspeed) (`self.CharacterMovement`)))

(fn `UserConstructionScript`
  (`parent.UserConstructionScript`))