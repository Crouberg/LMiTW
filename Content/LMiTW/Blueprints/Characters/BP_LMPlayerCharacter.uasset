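; Player character Blueprint that handles input, view switching and camera look, starting in first person with a toggle to third person.
; Key states for crouch, run, crawl and antigravity feed a player control movement component through the Move Forward axis event, though crawl has no live binding.
; A PDA key toggles a flag.
; Overridable-style functions supply footstep audio, animation references and movement/stamina settings, while CanMove always allows movement.
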(event `self.ReceiveBeginPlay`
  ;[1 1 1] BeginPlay
  ;[1 1 1] SetDefaultCamera
  (`ActorComponent.SetActive` (`self.CameraFirstPerson`) true false)
  (`ActorComponent.SetActive` (`self.CameraComponent`) false false)
  (`ActorComponent.SetActive` (`self.CameraThirdPerson`) false false))

(event `Key|V`
  (params (Key :type "Key Structure"))
  ;[1 1 1] Swtich view camera
  (:`Pressed`
    (`/Engine/EditorBlueprintResources/StandardMacros.FlipFlop`
      (:`A`
        (`ActorComponent.SetActive` (`self.CameraThirdPerson`) true false)
        (`ActorComponent.SetActive` (`self.CameraFirstPerson`) false false))
      (:`B`
        (`ActorComponent.SetActive` (`self.CameraFirstPerson`) true false)
        (`ActorComponent.SetActive` (`self.CameraThirdPerson`) false false)))))

(event `InputAxis|Move Forward`
  (params (AxisValue :type "Float (single-precision)"))
  ;[1 1 1] Movement
  (message `/Game/LMiTW/Blueprints/Interface/BPI_Movement.PlayerInput` (`self.BP_PlayerControlMovementComponent`) AxisValue (stale `InputAxis|Move Right` AxisValue) (`self.PressKeyCrouch?`) (`self.PressKeyRun?`) (`self.PressKeyCrowl?`) (`self.PressKeyAntiGravityMode?`) false (not (`self.CanMove`))))

(event `InputAxis|Move Right`
  (params (AxisValue :type "Float (single-precision)"))
  ;[1 1 1] Movement
)

(event `InputAxis|Turn`
  (params (AxisValue :type "Float (single-precision)"))
  ;[1 1 1] Mouse
  (bind _output_get (set `self.YawDirection` AxisValue))
  (`self.AddControllerYawInput` _output_get))

(event `InputAxis|LookUp`
  (params (AxisValue :type "Float (single-precision)"))
  ;[1 1 1] Mouse
  (bind _output_get (set `self.PitchDirection` AxisValue))
  (`self.AddControllerPitchInput` _output_get))

(event `Key|LeftControl`
  (params (Key :type "Key Structure"))
  ;[1 1 1] crouch
  (:`Pressed`
    (set `self.PressKeyCrouch?` true :!label _label))
  (:`Released`
    (set `self.PressKeyCrouch?` false :!label _label_2)))

(event `Key|K`
  (params (Key :type "Key Structure"))
  ;[1 1 1] antigravityMode
  (:`Pressed`
    (set `self.PressKeyAntiGravityMode?` true))
  (:`Released`
    (set `self.PressKeyAntiGravityMode?` false)))

(event `Key|C`
  (params (Key :type "Key Structure"))
  ;[1 1 1] crouch
  (:`Pressed`
    (goto _label))
  (:`Released`
    (goto _label_2)))

(event `Key|F`
  (params (Key :type "Key Structure"))
  ;[1 1 1] PDA
  (:`Pressed`
    (`/Engine/EditorBlueprintResources/StandardMacros.FlipFlop`
      (:`A`
        (set `self.PressKeyUsePDA?` true))
      (:`B`
        (set `self.PressKeyUsePDA?` false)))))

(event `Key|LeftShift`
  (params (Key :type "Key Structure"))
  ;[1 1 1] run
  (:`Pressed`
    (set `self.PressKeyRun?` true))
  (:`Released`
    (set `self.PressKeyRun?` false)))

(event `Key|Z`
  (params (Key :type "Key Structure"))
  ;[1 1 1] crowl
)

(fn `CanMove`
  (returns (Result :type Boolean))
  (return true))

(fn `GetSoundStepInfo`
  (returns (Success :type Boolean) (FootStepsAudioComponent :type "AudioComponent Object Reference") (`FootStepsPlay?` :type Boolean) (`EquipmentPlay?` :type Boolean) (FootStepsVolume :type "Float (double-precision)") (EquipmentVolume :type "Float (double-precision)") (`IsMale?` :type Boolean))
  (return true (`self.FootSteps`) true true 1.0 1.0 true))

(fn `InitializeAnimationParametrs`
  (returns (LMBase_Chracter :type "LMBaseCharacter Object Reference") (BP_ControlMovementComponent :type "/Game/LMiTW/Blueprints/Components/BP_PlayerControlMovementComponent Object Reference"))
  (return self (`self.BP_PlayerControlMovementComponent`)))

(fn `InitializeMovementParametrs`
  (returns (InitParametrs :type "/Game/LMiTW/Blueprints/Structures/S_MovementInitInfo Structure"))
  (return (`self.sMovementAndStamina`)))

(fn `UserConstructionScript`)