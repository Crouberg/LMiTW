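; Player interaction component that detects interactable actors in the first-person view of the owning BP_LMPlayerCharacter.
; A looping timer line-traces from the camera and accepts hit actors implementing BPI_Interactable.
; Target changes send start and stop focus messages and toggle the game overlay's cursor tooltip, shown only for named targets.
; Interact forwards the owner to the current target, and a debug flag enables trace drawing and logging.
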(event `self.ReceiveBeginPlay`
  ;[1 1 1] Init
  (`self.InitOwner`)
  (`self.StartTracing`))

(event `Interact`
  ;[1 1 1] Calls when player press the key for interaction
  (bind _currentinteractiontarget (`self.CurrentInteractionTarget`)
    (:`then`
      (message `/Game/LMiTW/Blueprints/Interface/BPI_Interactable.Interact` _currentinteractiontarget (`self.OwnerPlayerCharacter`)))
    (:`else`)))

(fn `ClearTarget`
  (bind _currentinteractiontarget (`self.CurrentInteractionTarget`)
    (:`then`
      (message `/Game/LMiTW/Blueprints/Interface/BPI_Interactable.StopFocus` _currentinteractiontarget)
      (if (`self.IsTraceDebugMode`)
        (`KismetSystemLibrary.PrintString` "ClearTarget()" true true (struct :`R` 0.324843 :`G` 1.0 :`B` 0.416074 :`A` 1.0))))
    (:`else`
      _))
  (`self.HideCursorTooltip`)
  (set `self.CurrentInteractionTarget` null))

(fn `GetTraceParams`
  (returns (Start :type "Vector Structure") (End :type "Vector Structure"))
  (bind _camerafirstperson (`/Game/LMiTW/Blueprints/Character/BP_LMPlayerCharacter.CameraFirstPerson` (`self.OwnerPlayerCharacter`)))
  (bind _returnvalue (`SceneComponent.K2_GetComponentLocation` _camerafirstperson))
  (return _returnvalue (+ _returnvalue (* (`SceneComponent.GetForwardVector` _camerafirstperson) (`self.TraceDistance`)))))

(fn `HaveInteractionText`
  (params (S_InteractionInfo :type "/Game/LMiTW/Blueprints/Structures/S_InteractionInfo Structure (by ref)"))
  (returns (ReturnValue :type Boolean))
  (return (`KismetTextLibrary.NotEqual_TextText` (`.Name_3_2CA896B84EC61FBC1CBB7C9044E1313A` (break `/Game/LMiTW/Blueprints/Structures/S_InteractionInfo` S_InteractionInfo)) "")))

(fn `HideCursorTooltip`
  (`/Game/LMiTW/HUD/GameOverlay/WBP_GameOverlay.HideCursorTooltip` (`/Game/LMiTW/Blueprints/FunctionLibrary/LMFunctionLibrary.GetGameOverlay`)))

(fn `InitOwner`
  (bind _asbp_lmplayer_character (cast `/Game/LMiTW/Blueprints/Character/BP_LMPlayerCharacter` (`self.GetOwner`)))
  (set `self.OwnerPlayerCharacter` _asbp_lmplayer_character))

(fn `SetTarget`
  (params (NewTarget :type "Actor Object Reference"))
  (`self.ClearTarget`)
  (bind _output_get (set `self.CurrentInteractionTarget` NewTarget))
  (message `/Game/LMiTW/Blueprints/Interface/BPI_Interactable.StartFocus` _output_get)
  (`self.ShowCursorTooltip`)
  (if (`self.IsTraceDebugMode`)
    (`KismetSystemLibrary.PrintString` "SetTarget()" true true (struct :`R` 0.324843 :`G` 1.0 :`B` 0.416074 :`A` 1.0))))

(fn `ShowCursorTooltip`
  (bind _info (message `/Game/LMiTW/Blueprints/Interface/BPI_Interactable.GetInteractInfo` (`self.CurrentInteractionTarget`)))
  (if (`self.HaveInteractionText` _info)
    (`/Game/LMiTW/HUD/GameOverlay/WBP_GameOverlay.ShowCursorTooltip` (`/Game/LMiTW/Blueprints/FunctionLibrary/LMFunctionLibrary.GetGameOverlay`) _info)))

(fn `StartTracing`
  (bind _returnvalue (`KismetSystemLibrary.K2_SetTimer` null "TraceForInteract" (`self.TraceInterval`) true))
  (set `self.InteractionTimer` _returnvalue))

(fn `StopTracing`
  (`KismetSystemLibrary.K2_ClearAndInvalidateTimerHandle` (`self.InteractionTimer`))
  (`self.ClearTarget`))

(fn `TraceForInteract`
  (locals (L_PotentialTarget :type "Actor Object Reference"))
  (bind (_start _end) (`self.GetTraceParams`))
  (bind (_outhit _returnvalue) (`KismetSystemLibrary.LineTraceSingle` :`Start` _start :`End` _end :`TraceChannel` "TraceTypeQuery3" :`DrawDebugType` (select `bool` (`self.IsTraceDebugMode`) :`true` "ForDuration" :!type "EDrawDebugTrace Enum") :`TraceColor` (struct :`R` 1.0 :`G` 0.94821 :`B` 0.113053 :`A` 1.0) :`DrawTime` (`self.DebugLineDuration`)))
  (if _returnvalue
    (bind _output_get (set `local.L_PotentialTarget` (`.HitActor` (`GameplayStatics.BreakHitResult` _outhit))))
    (if (!= _output_get (`self.CurrentInteractionTarget`))
      (bind _success (`self.ValidateTarget` (`local.L_PotentialTarget`)))
      (if _success
        (`self.SetTarget` (`local.L_PotentialTarget`))
        (else
          (`self.ClearTarget`)))
      (else
        (return)))
    (else
      (`self.ClearTarget`) ; Not hit - clearing target!
      (return))))

(fn `ValidateTarget`
  (params (Target :type "Actor Object Reference"))
  (returns (Success :type Boolean))
  (if (`KismetSystemLibrary.DoesImplementInterface` Target "/Game/LMiTW/Blueprints/Interface/BPI_Interactable.BPI_Interactable_C")
    (return true)
    (else
      (return false))))