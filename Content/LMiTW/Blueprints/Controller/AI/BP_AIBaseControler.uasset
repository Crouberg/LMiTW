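; Base AI controller that drives an enemy hunting the player through staged behavior trees and an enum mode.
; On BeginPlay it reads start stage and mode from the pawn via messages, runs that stage's tree and sets up the blackboard.
; Perception updates set the target player or last stimulus location, switching modes mirrored to blackboard and pawn.
; Patrol points are random reachable locations around the player, with capped retries and a zero-vector fallback.
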(event `self.ReceiveBeginPlay`
  (`self.Init`))

(event `self.Perception.OnPerceptionUpdated`
  (params (UpdatedActors :type "Array of Actor Object Reference (by ref)"))
  (`self.ProcessSences` UpdatedActors))

(event `/Game/LMiTW/Blueprints/Interface/BPI_AIController.TargetReached`
  (params (Target :type "Actor Object Reference"))
  (if (`self.ActorHasTag` Target "Player")
    (`self.SetMode` "NewEnumerator2")))

(event `self.Perception.OnTargetPerceptionInfoUpdated`
  (params (UpdateInfo :type "ActorPerceptionUpdateInfo Structure (by ref)"))
  (`self.UpdatePerception` UpdateInfo))

(event `InspectingEnded`
  ;[1 1 1] Inspecting end
  (`self.SetMode` "NewEnumerator1"))

(event `/Game/LMiTW/Blueprints/Interface/BPI_AIController.IncrementInspectingIteration`
  ;[1 1 1] Inspect iterations
  (`self.IncrementInspectingIterations`))

(fn `GetAcceptablePatrolPoint`
  (returns (Success :type Boolean) (Point :type "Vector Structure"))
  (bind _distance (message `/Game/LMiTW/Blueprints/Interface/BPI_AICharacter.GetAcceptableDistance` (`self.K2_GetPawn`)))
  (bind (_randomlocation _returnvalue) (`NavigationSystemV1.K2_GetRandomReachablePointInRadius` (`self.K2_GetActorLocation` (`GameplayStatics.GetPlayerCharacter` 0)) _distance null null))
  (return _returnvalue _randomlocation))

(fn `GetAIMode`
  (returns (Mode :type "/Game/LMiTW/Blueprints/Enums/E_AIMode Enum"))
  (return (`self.GetMode`)))

(fn `GetMode`
  (returns (Mode :type "/Game/LMiTW/Blueprints/Enums/E_AIMode Enum"))
  (return (`self.CurrentMode`)))

(fn `GetNewPatrolPoint`
  (returns (Point :type "Vector Structure"))
  (return (`self.GetNextPatrolPoint`)))

(fn `GetNextPatrolPoint`
  (returns (Point :type "Vector Structure"))
  (locals (Local_SearchFails :type Integer) (Local_MaxSearchFails :type Integer :default 100))
  (bind (_success _point) (`self.GetAcceptablePatrolPoint`))
  (if (< (`local.Local_SearchFails`) (`local.Local_MaxSearchFails`)) :!label _label
    (if _success
      (return _point)
      (else
        (`/Engine/EditorBlueprintResources/StandardMacros.IncrementInt` (`local.Local_SearchFails`) ; Infinity loop protecting
          (:`  `
            (goto _label)))))
    (else
      (return (0.0 0.0 0.0)) ; Fail - returns zero location. TODO Add fail handling
    )))

(fn `GetStartMode`
  (returns (Mode :type "/Game/LMiTW/Blueprints/Enums/E_AIMode Enum"))
  (`/Engine/EditorBlueprintResources/StandardMacros.IsValid` (`self.K2_GetPawn`)
    (:`Is Valid`
      (bind _mode (message `/Game/LMiTW/Blueprints/Interface/BPI_AICharacter.GetStartMode` (`self.K2_GetPawn`)))
      (return _mode))
    (:`Is Not Valid`
      (return "NewEnumerator0"))))

(fn `GetStartStage`
  (returns (Stage :type "/Game/LMiTW/Blueprints/Enums/E_AIStages Enum"))
  (bind _returnvalue (`self.K2_GetPawn`))
  (`/Engine/EditorBlueprintResources/StandardMacros.IsValid` _returnvalue
    (:`Is Valid`
      (bind _stage (message `/Game/LMiTW/Blueprints/Interface/BPI_AICharacter.GetStartStage` _returnvalue))
      (return _stage))
    (:`Is Not Valid`
      (return "NewEnumerator0"))))

(fn `IncrementInspectingIterations`
  (if (< (`self.CurrentInspectingIterations`) (`self.MaxInspectingIterations`))
    (`/Engine/EditorBlueprintResources/StandardMacros.IncrementInt` (`self.CurrentInspectingIterations`))
    (else
      (set `self.CurrentInspectingIterations` 0)
      (`self.InspectingEnded`))))

(fn `Init`
  (`self.SetStage` (`self.GetStartStage`))
  (`self.SetMode` (`self.GetStartMode`))
  (`self.UseBlackboard` (`self.DefaultBlackboard`))
  (`BlackboardComponent.SetValueAsObject` (`self.Blackboard`) "Controller" self))

(fn `ProcessSences`
  (params (Targets :type "Array of Actor Object Reference"))
  (for _array_element Targets
    (if (`self.ActorHasTag` _array_element "Player")
      (`self.SetTargetPlayer` _array_element)
      (`self.SetMode` "NewEnumerator5"))))

(fn `SetInspectingLocation`
  (params (Location :type "Vector Structure"))
  (bind _output_get (set `self.InspectLocation` Location))
  (`BlackboardComponent.SetValueAsVector` (`self.Blackboard`) "InspectingLocation" _output_get))

(fn `SetMode`
  (params (Mode :type "/Game/LMiTW/Blueprints/Enums/E_AIMode Enum" :default "NewEnumerator0"))
  (bind _output_get (set `self.CurrentMode` Mode))
  (`BlackboardComponent.SetValueAsEnum` (`self.Blackboard`) "CurrentMode" _output_get)
  (message `/Game/LMiTW/Blueprints/Interface/BPI_AICharacter.SetMode` (`self.K2_GetPawn`) (`self.GetMode`)))

(fn `SetSensesSetup`
  (params (NewSetup :type "/Game/LMiTW/Blueprints/Structures/S_AISensesSetup Structure")))

(fn `SetStage`
  (params (Stage :type "/Game/LMiTW/Blueprints/Enums/E_AIStages Enum" :default "NewEnumerator0"))
  (returns (Success :type Boolean))
  (bind _output_get (set `self.CurrentStage` Stage))
  (switch `/Game/LMiTW/Blueprints/Enums/E_AIStages` _output_get
    (:`NewEnumerator0`
      (`KismetSystemLibrary.PrintString` "AI - Setted a not valid stage!" true true (struct :`R` 1.0 :`B` 0.008603 :`A` 1.0) 5.0)
      (`self.RunBehaviorTree` null)
      (return false))
    (:`NewEnumerator1`
      (bind _returnvalue (`self.RunBehaviorTree` (`self.BehaviorTreeStageFirst`)))
      (return _returnvalue))
    (:`NewEnumerator2`
      (bind _returnvalue_2 (`self.RunBehaviorTree` (`self.BehaviorTreeStageSecond`)))
      (return _returnvalue_2))
    (:`NewEnumerator3`
      (bind _returnvalue_3 (`self.RunBehaviorTree` (`self.BehaviorTreeStageThird`)))
      (return _returnvalue_3))))

(fn `SetTargetPlayer`
  (params (Target :type "Actor Object Reference"))
  (bind _output_get (set `self.TargetPlayer` Target))
  (`BlackboardComponent.SetValueAsObject` (`self.Blackboard`) "TargetPlayer" _output_get))

(fn `StartPatrol`
  (`self.SetMode` "NewEnumerator1"))

(fn `UpdatePerception`
  (params (ActorPerceptionUpdateInfo :type "ActorPerceptionUpdateInfo Structure (by ref)"))
  (bind (_targetid _target _stimulus) (break `ActorPerceptionUpdateInfo` ActorPerceptionUpdateInfo))
  (bind ((`StimulusLocation` _stimuluslocation) (`bSuccessfullySensed` _bsuccessfullysensed)) (break `AIStimulus` _stimulus))
  (if (`self.ActorHasTag` _target "Player")
    (if (not _bsuccessfullysensed)
      (`self.SetInspectingLocation` _stimuluslocation)
      (`self.SetMode` "NewEnumerator6"))))

(fn `UserConstructionScript`)