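; Blueprint function library of shared helpers for overlay access, spawn transforms and item lookup.
; GetGameOverlay asks player controller 0 for its game overlay, and GetZeroSpawnTransform returns an origin transform with unit scale.
; GetItemFromTableByID linearly scans DT_Items rows, matching the Id field rather than the row name.
; It stops at the first match and has no explicit not-found result.
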(fn `GetGameOverlay`
  (returns (GameOverlayWidget :type "/Game/LMiTW/HUD/GameOverlay/WBP_GameOverlay Object Reference"))
  (bind _gameoverlaywidget (message `/Game/LMiTW/Blueprints/Interface/BPI_PlayerController.GetGameOverlay` (`GameplayStatics.GetPlayerController` (`local.__WorldContext`))))
  (return _gameoverlaywidget))

(fn `GetItemFromTableByID`
  (params (Id :type Integer))
  (returns (ItemInfo :type "/Game/LMiTW/Blueprints/Structures/S_ItemInfo Structure"))
  (locals (LocalID :type Integer) (LocalItem :type "/Game/LMiTW/Blueprints/Structures/S_ItemInfo Structure"))
  (set `local.LocalID` Id)
  (bind _outrownames (`DataTableFunctionLibrary.GetDataTableRowNames` "/Game/LMiTW/Data/Items/DT_Items.DT_Items"))
  (for _array_element _outrownames
    (bind _returnvalue (`|GetDataTableRow` "/Game/LMiTW/Data/Items/DT_Items.DT_Items" _array_element)
      (:`then`
        (if (== (`.Id_26_B8349D294FC6345E116DB081DF9569FA` (break `/Game/LMiTW/Blueprints/Structures/S_ItemInfo` _returnvalue)) (`local.LocalID`))
          (set `local.LocalItem` _returnvalue)
          (break)))))
  (return (`local.LocalItem`)))

(fn `GetZeroSpawnTransform`
  (returns (Transform :type "Transform Structure"))
  (return (`KismetMathLibrary.MakeTransform` (0.0 0.0 0.0))))