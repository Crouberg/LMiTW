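; BP_InteractableActor is an interactable actor that accepts a two-handed item named "Acum" from the player or other interactor.
; On Interact, it checks the held item's name, has the interactor drop it, sets HaveApplyItem and attaches the item to ItemSocket.
; Focus events toggle custom depth on the static mesh, whose asset the construction script takes from ItemInfo.
; ApplyItem is an empty stub, and GetInteractInfo returns stored interaction info.
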(event `/Game/LMiTW/Blueprints/Interface/BPI_Interactable.Interact`
  (params (Interactor :type "/Game/LMiTW/Blueprints/Character/BP_LMPlayerCharacter Object Reference"))
  (bind (_haveitem_ _iteminfo _actor) (`/Game/LMiTW/Blueprints/Character/BP_LMPlayerCharacter.GetTwoHandedItem` Interactor))
  (if _haveitem_
    (if (`KismetTextLibrary.EqualEqual_TextText` "Acum" (`.Name_2_C87A6EC948CB0F82780F01BD265E0887` (break `/Game/LMiTW/Blueprints/Structures/S_ItemInfo` _iteminfo)))
      (`/Game/LMiTW/Blueprints/Character/BP_LMPlayerCharacter.DropTwoHandedItem` Interactor false)
      (set `self.HaveApplyItem?` true)
      (bind _output_get (set `self.Item` _actor))
      (`self.K2_AttachToActor` _output_get self "ItemSocket" "SnapToTarget" "KeepRelative" "KeepWorld" true))))

(event `/Game/LMiTW/Blueprints/Interface/BPI_Interactable.StartFocus`
  (`self.SetRenderCustomDepth` true))

(event `/Game/LMiTW/Blueprints/Interface/BPI_Interactable.StopFocus`
  (`self.SetRenderCustomDepth` false))

(fn `ApplyItem`)

(fn `GetInteractInfo`
  (returns (Info :type "/Game/LMiTW/Blueprints/Structures/S_InteractionInfo Structure"))
  (return (`self.InteractInfo`)))

(fn `SetRenderCustomDepth`
  (params (Render :type Boolean))
  (`PrimitiveComponent.SetRenderCustomDepth` (`self.StaticMesh`) Render))

(fn `UserConstructionScript`
  (`StaticMeshComponent.SetStaticMesh` (`self.StaticMesh`) (`.StaticMesh_23_9F5223F84DD7D2895F9C5585A125810E` (break `/Game/LMiTW/Blueprints/Structures/S_ItemInfo` (`self.ItemInfo`)))))