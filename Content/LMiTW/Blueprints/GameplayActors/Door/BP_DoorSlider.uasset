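; Sliding door actor that extends a parent door class and moves its mesh sideways to open and close.
; On init it caches the closed position, derives the open one from an offset along local Y and applies the opening speed to a timeline.
; That timeline linearly interpolates the mesh between both positions, playing forward to open and reversing to close.
; Indirect access activation and deactivation either open/close or lock/unlock the door, depending on its mode.
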(event `self.PlayOpeningAnimation`
  ;[1 1 1] Animation
  (bind (_direction _alpha) (`Timeline|AnimationTimeline` :!label _label)
    (:`Update`
      (`self.MoveDoorMesh` (`self.GetNewLocation` _alpha)))))

(event `self.PlayClosingAnimation`
  ;[1 1 1] Animation
  (goto _label :!via `Reverse`))

(fn `GetNewLocation`
  (params (Alpha :type "Float (double-precision)"))
  (returns (Location :type "Vector Structure"))
  (return (`|EaseFunction` "Linear" Alpha (`self.ClosedLocation`) (`self.OpenedLocation`))))

(fn `IndirectAccessActivate`
  (`parent.IndirectAccessActivate`)
  (switch `/Game/LMiTW/Blueprints/Enums/E_DoorIndirectControlMode` (`self.IndirectAccessMode`)
    (:`NewEnumerator1`
      (`self.OpenDoor` null))
    (:`NewEnumerator2`
      (`self.LockDoor`))))

(fn `IndirectAccessDeactivate`
  (`parent.IndirectAccessDeactivate`)
  (switch `/Game/LMiTW/Blueprints/Enums/E_DoorIndirectControlMode` (`self.IndirectAccessMode`)
    (:`NewEnumerator1`
      (`self.CloseDoor` null))
    (:`NewEnumerator2`
      (`self.UnlockDoor`))))

(fn `Init`
  ;[1 1 1] TODO: Переделать весь этот бардак
  (`parent.Init`)
  (`self.InitDoorMeshLocations`)
  (`TimelineComponent.SetPlayRate` (`self.AnimationTimeline`) (`self.OpeningSpeed`)))

(fn `InitDoorMeshLocations`
  (bind _output_get (set `self.ClosedLocation` (`SceneComponent.RelativeLocation` (`self.DoorMesh`))))
  (set `self.OpenedLocation` (`KismetMathLibrary.MakeVector` (.x _output_get) (- (.y _output_get) (`self.Offset`)) (.z _output_get))) ; Just add some offset to door mesh base (closed) location
)

(fn `MoveDoorMesh`
  (params (NewLocation :type "Vector Structure"))
  (`SceneComponent.K2_SetRelativeLocation` (`self.DoorMesh`) NewLocation false false))

(fn `UserConstructionScript`
  (`parent.UserConstructionScript`))