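; BP_DoorSlider_Big is a sliding door actor that opens by lowering its mesh along local Z.
; Init caches the closed location, subtracts an offset for the open one, and sets the timeline play rate from the opening speed.
; Opening plays the timeline to linearly interpolate the mesh between both locations, and closing reverses it.
; A helper identifies linked master switchers as control panel or button classes, printing an error otherwise.
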(event `self.PlayOpeningAnimation`
  ;[1 1 1] Animation
  (bind (_direction _alpha) (`Timeline|AnimationTimeline` :!label _label)
    (:`Update`
      (`self.MoveDoorMesh` (`self.GetNewLocation` _alpha)))))

(event `self.PlayClosingAnimation`
  ;[1 1 1] Animation
  (goto _label :!via `Reverse`))

(event `/Game/LMiTW/Blueprints/Interface/BPI_Generator.SetSwitcherReferencesToDoor`
  (params (SelfActor :type "Actor Object Reference"))
  (`parent.SetSwitcherReferencesToDoor` SelfActor))

(fn `GetNewLocation`
  (params (Alpha :type "Float (double-precision)"))
  (returns (Location :type "Vector Structure"))
  (return (`|EaseFunction` "Linear" Alpha (`self.ClosedLocation`) (`self.OpenedLocation`))))

(fn `Init`
  ;[1 1 1] TODO: Переделать весь этот бардак
  (`parent.Init`)
  (`self.InitDoorMeshLocations`)
  (`TimelineComponent.SetPlayRate` (`self.AnimationTimeline`) (`self.OpeningSpeed`)))

(fn `InitDoorMeshLocations`
  (bind _output_get (set `self.ClosedLocation` (`SceneComponent.RelativeLocation` (`self.Door`))))
  (set `self.OpenedLocation` (`KismetMathLibrary.MakeVector` (.x _output_get) (.y _output_get) (- (.z _output_get) (`self.OpeningOffset`)))) ; Just add some offset to door mesh base (closed) location
)

(fn `MoveDoorMesh`
  (params (NewLocation :type "Vector Structure"))
  (`SceneComponent.K2_SetRelativeLocation` (`self.Door`) NewLocation false false))

(fn `UserConstructionScript`
  (`parent.UserConstructionScript`))

(fn `WhatSubsidiaryClassOfMasterSwitcher`
  (returns (SubsidiaryClass :type "/Game/LMiTW/Blueprints/GameplayActors/Switcher/BP_MasterSwitcher Class Reference"))
  (for _array_element (`self.BP_MasterSwitchers`)
    (bind _asbp_door_control_panel (cast `/Game/LMiTW/Blueprints/GameplayActors/Switcher/BP_DoorControlPanel` _array_element))
    (return (`GameplayStatics.GetObjectClass` _asbp_door_control_panel)))
  (bind _asbp_button (cast `/Game/LMiTW/Blueprints/GameplayActors/Switcher/BP_Button` _array_element)
    (:`then`
      (return (`GameplayStatics.GetObjectClass` _asbp_button)))
    (:`CastFailed`
      (`KismetSystemLibrary.PrintString` (`KismetStringLibrary.Concat_StrStr` (`KismetSystemLibrary.GetObjectName` self) ": WhatSubsidiaryClassOfMasterSwitcher function. ERR. Wrong classes or another mistake") true true (struct :`R` 1.0 :`B` 0.057804 :`A` 1.0) 20.0))))