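; Base door actor that opens, closes and locks, with animation, init and indirect-access hooks left empty, apparently for child Blueprints.
; In auto mode, overlaps on the activation box, sized in the construction script, trigger opening and closing.
; Opening and closing call notifications and animation events, but the lock blocks only opening.
; Controlled-actor events forward console or switcher signals to the access hooks, and helpers expose interaction info and mesh custom depth.
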(event `self.ReceiveBeginPlay`
  ;[1 1 1] Init
  (`self.Init`))

(event `self.ActivationVolumeBox.OnComponentBeginOverlap`
  (params (OverlappedComponent :type "PrimitiveComponent Object Reference") (OtherActor :type "Actor Object Reference") (OtherComp :type "PrimitiveComponent Object Reference") (OtherBodyIndex :type Integer) (bFromSweep :type Boolean) (SweepResult :type "HitResult Structure (by ref)"))
  ;[1 1 1] Open / close
  (if (`self.IsAutoOneningMode`)
    (`self.OpenDoor` null)))

(event `self.ActivationVolumeBox.OnComponentEndOverlap`
  (params (OverlappedComponent :type "PrimitiveComponent Object Reference") (OtherActor :type "Actor Object Reference") (OtherComp :type "PrimitiveComponent Object Reference") (OtherBodyIndex :type Integer))
  ;[1 1 1] Open / close
  (if (`self.IsAutoOneningMode`)
    (`self.CloseDoor` null)))

(event `PlayOpeningAnimation`
  ;[1 1 1] Open / close
  ;;[0.6146 1 0.6667] Animation
)

(event `PlayClosingAnimation`
  ;[1 1 1] Open / close
  ;;[0.6146 1 0.6667] Animation
)

(event `/Game/LMiTW/Blueprints/Interface/BPI_IndirectAccess.ActivateControlledActor`
  ;[1 1 1] Open / close
  ;;[0.5395 1 0.5982] Indirect access (via console or switcher) - if connected
  (`self.IndirectAccessActivate`))

(event `/Game/LMiTW/Blueprints/Interface/BPI_IndirectAccess.DeactivateControlledActor`
  ;[1 1 1] Open / close
  ;;[0.5395 1 0.5982] Indirect access (via console or switcher) - if connected
  (`self.IndirectAccessDeactivate`))

(fn `CloseDoor`
  (params (Instigator :type "Actor Object Reference"))
  (`self.OnDoorClosed` Instigator)
  (`self.PlayClosingAnimation`))

(fn `GetInteractInfo`
  (returns (Info :type "/Game/LMiTW/Blueprints/Structures/S_InteractionInfo Structure"))
  (return (`self.InteractInfo`)))

(fn `IndirectAccessActivate`)

(fn `IndirectAccessDeactivate`)

(fn `Init`)

(fn `LockDoor`
  (set `self.IsLocked` true))

(fn `OpenDoor`
  (params (Instigator :type "Actor Object Reference"))
  (if (not (`self.IsLocked`))
    (`self.OnDoorOpened` Instigator)
    (`self.PlayOpeningAnimation`)
    (else
      (return))))

(fn `SetActivationBoxExtents`
  (`BoxComponent.SetBoxExtent` (`self.ActivationVolumeBox`) (`self.ActivationBoxExtent`) true))

(fn `SetDoorMode`
  (params (IsAutoMode :type Boolean))
  (set `self.IsAutoOneningMode` IsAutoMode))

(fn `SetRenderCustomDepth`
  (params (Render :type Boolean))
  (`PrimitiveComponent.SetRenderCustomDepth` (`self.DoorMesh`) Render))

(fn `UnlockDoor`
  (set `self.IsLocked` false))

(fn `UserConstructionScript`
  (`self.SetActivationBoxExtents`))