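; Default item pickup actor that players interact with to add an item to their storage.
; PreInit looks up item info by ItemId, clamps the count to the item's stack size and applies the static mesh, while Init copies the item name into the interaction info.
; PickUp tries adding the item to the interactor's BP_PlayerStorageComponent and, on success, destroys the pickup through a short lifespan.
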(fn `ClampToStackSize`
  (params (ItemInfo :type "/Game/LMiTW/Blueprints/Structures/S_ItemInfo Structure (by ref)"))
  (bind ((`Count_17_D19A6EBD41C242C28CC0F39910C423A9` _count) (`StackSize_22_A0B76A20497498BC51DB029EFCFB634F` _stacksize)) (break `/Game/LMiTW/Blueprints/Structures/S_ItemInfo` ItemInfo))
  (bind _structout (setmembers `/Game/LMiTW/Blueprints/Structures/S_ItemInfo` :`StructRef` ItemInfo :`Count` (`KismetMathLibrary.Clamp` _count 1 _stacksize)))
  (set `self.Count` (`.Count_17_D19A6EBD41C242C28CC0F39910C423A9` (break `/Game/LMiTW/Blueprints/Structures/S_ItemInfo` _structout))))

(fn `Init`
  (`parent.Init`)
  (setmembers `/Game/LMiTW/Blueprints/Structures/S_InteractionInfo` :`StructRef` (`self.InteractInfo`) :`Name` (`.Name_2_C87A6EC948CB0F82780F01BD265E0887` (break `/Game/LMiTW/Blueprints/Structures/S_ItemInfo` (`self.ItemInfo`)))))

(fn `PickUp`
  (params (Interactor :type "/Game/LMiTW/Blueprints/Character/BP_LMPlayerCharacter Object Reference"))
  (bind _returnvalue (`self.GetComponentByClass` Interactor "/Game/LMiTW/Blueprints/Components/BP_PlayerStorageComponent.BP_PlayerStorageComponent_C"))
  (`parent.PickUp` Interactor)
  (`/Engine/EditorBlueprintResources/StandardMacros.IsValid` _returnvalue
    (:`Is Valid`
      (bind _success (`/Game/LMiTW/Blueprints/Components/BP_PlayerStorageComponent.TryAddItem` _returnvalue (`self.ItemInfo`)))
      (if _success
        (`self.SetLifeSpan` 0.1)))))

(fn `PreInit`
  (`parent.PreInit`)
  (bind _output_get (set `self.ItemInfo` (`/Game/LMiTW/Blueprints/FunctionLibrary/LMFunctionLibrary.GetItemFromTableByID` (`self.ItemId`))))
  (bind _structout (setmembers `/Game/LMiTW/Blueprints/Structures/S_ItemInfo` :`StructRef` _output_get :`Count` (`self.Count`)))
  (`self.ClampToStackSize` _structout)
  (`StaticMeshComponent.SetStaticMesh` (`self.PickupMesh`) (`.StaticMesh_23_9F5223F84DD7D2895F9C5585A125810E` (break `/Game/LMiTW/Blueprints/Structures/S_ItemInfo` (`self.ItemInfo`)))))

(fn `UserConstructionScript`
  (`parent.UserConstructionScript`))