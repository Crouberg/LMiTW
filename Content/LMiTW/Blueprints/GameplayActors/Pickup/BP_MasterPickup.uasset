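; Base pickup actor that places a data-table item in the world for the player to collect.
; The construction script looks up ItemId, applies Count and sets the item's mesh; BeginPlay copies the item name into its interaction info.
; Interact offers the item to the interactor's BP_PlayerStorageComponent and, on success, expires the actor after a short lifespan.
; Focus events toggle custom depth on the mesh for highlighting.
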(event `self.ReceiveBeginPlay`
  (`self.Init`))

(event `/Game/LMiTW/Blueprints/Interface/BPI_Interactable.Interact`
  (params (Interactor :type "/Game/LMiTW/Blueprints/Character/BP_LMPlayerCharacter Object Reference"))
  ;[1 1 1] Pick up
  (`self.PickUp` Interactor))

(event `/Game/LMiTW/Blueprints/Interface/BPI_Interactable.StartFocus`
  ;[1 1 1] Focusing
  (`self.SetRenderCustomDepth` true))

(event `/Game/LMiTW/Blueprints/Interface/BPI_Interactable.StopFocus`
  ;[1 1 1] Focusing
  (`self.SetRenderCustomDepth` false))

(fn `GetInteractInfo`
  (returns (Info :type "/Game/LMiTW/Blueprints/Structures/S_InteractionInfo Structure"))
  (return (`self.InteractInfo`)))

(fn `Init`
  (setmembers `/Game/LMiTW/Blueprints/Structures/S_InteractionInfo` :`StructRef` (`self.InteractInfo`) :`Name` (`.Name_2_C87A6EC948CB0F82780F01BD265E0887` (break `/Game/LMiTW/Blueprints/Structures/S_ItemInfo` (`self.ItemInfo`)))))

(fn `PickUp`
  (params (Interactor :type "LMPlayerCharacter Object Reference"))
  (bind _returnvalue (`self.GetComponentByClass` Interactor "/Game/LMiTW/Blueprints/Components/BP_PlayerStorageComponent.BP_PlayerStorageComponent_C"))
  (`/Engine/EditorBlueprintResources/StandardMacros.IsValid` _returnvalue
    (:`Is Valid`
      (bind _success (`/Game/LMiTW/Blueprints/Components/BP_PlayerStorageComponent.TryAddItem` _returnvalue (`self.ItemInfo`)))
      (if _success
        (`self.SetLifeSpan` 0.1)))))

(fn `PreInit`
  (bind _output_get (set `self.ItemInfo` (`/Game/LMiTW/Blueprints/FunctionLibrary/LMFunctionLibrary.GetItemFromTableByID` (`self.ItemId`))))
  (setmembers `/Game/LMiTW/Blueprints/Structures/S_ItemInfo` :`StructRef` _output_get :`Count` (`self.Count`))
  (`StaticMeshComponent.SetStaticMesh` (`self.PickupMesh`) (`.StaticMesh_23_9F5223F84DD7D2895F9C5585A125810E` (break `/Game/LMiTW/Blueprints/Structures/S_ItemInfo` (`self.ItemInfo`)))))

(fn `SetRenderCustomDepth`
  (params (Render :type Boolean))
  (`PrimitiveComponent.SetRenderCustomDepth` (`self.PickupMesh`) Render))

(fn `UserConstructionScript`
  (`self.PreInit`))