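; BP_Note is a pickup actor for a readable note in the world.
; Interacting calls PickUp, which sends the interactor an ENoteOpen call with its NoteData and a reference to itself.
; Focus events toggle custom depth on PickupMesh for highlighting, and getters and a setter expose the note data and interaction info.
; Init and PreInit are empty hooks run from BeginPlay and the construction script.
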(event `self.ReceiveBeginPlay`
  (`self.Init`))

(event `/Game/LMiTW/Blueprints/Interface/BPI_Interactable.Interact`
  (params (Interactor :type "/Game/LMiTW/Blueprints/Character/BP_LMPlayerCharacter Object Reference") (InputKey :type "Key Structure"))
  ;[1 1 1] Pick up
  (`self.PickUp` Interactor))

(event `/Game/LMiTW/Blueprints/Interface/BPI_Interactable.StartFocus`
  ;[1 1 1] Focusing
  (`self.SetRenderCustomDepth` true))

(event `/Game/LMiTW/Blueprints/Interface/BPI_Interactable.StopFocus`
  ;[1 1 1] Focusing
  (`self.SetRenderCustomDepth` false))

(fn `GetInteractInfo`
  (returns (Info :type "/Game/LMiTW/Blueprints/Structures/S_InteractionInfo Structure"))
  (return (`self.InteractInfo`)))

(fn `GetNoteData`
  (returns (NoteData :type "/Game/LMiTW/Blueprints/Structures/S_NoteData Structure"))
  (return (`self.NoteData`)))

(fn `Init`)

(fn `PickUp`
  (params (Interactor :type "/Game/LMiTW/Blueprints/Character/BP_LMPlayerCharacter Object Reference"))
  (`/Game/LMiTW/Blueprints/Character/BP_LMPlayerCharacter.E_NoteOpen` Interactor (`self.NoteData`) self))

(fn `PreInit`)

(fn `SetNoteData`
  (params (NoteData :type "/Game/LMiTW/Blueprints/Structures/S_NoteData Structure"))
  (set `self.NoteData` NoteData))

(fn `SetRenderCustomDepth`
  (params (Render :type Boolean))
  (`PrimitiveComponent.SetRenderCustomDepth` (`self.PickupMesh`) Render))

(fn `UserConstructionScript`
  (`self.PreInit`))