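; Two-handed pickup item that an interactor can take and later drop, with its mesh set from ItemInfo in the construction script.
; The mesh simulates physics from BeginPlay, and dropping clears the in-use flag and sets physics as the caller requests.
; PickUp hands the item to the interactor through BPI_PlayerInteraction, marking it in use only if that call succeeds.
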(event `self.ReceiveBeginPlay`
  (`parent.ReceiveBeginPlay`)
  (`PrimitiveComponent.SetSimulatePhysics` (`self.PickupMesh`) true))

(event `self.PickUp`
  (params (Interactor :type "/Game/LMiTW/Blueprints/Character/BP_LMPlayerCharacter Object Reference"))
  (if (and (not (`self.InUse?`)) (`KismetSystemLibrary.DoesImplementInterface` Interactor "/Game/LMiTW/Blueprints/Interface/BPI_PlayerInteraction.BPI_PlayerInteraction_C"))
    (bind _success_ (message `/Game/LMiTW/Blueprints/Interface/BPI_PlayerInteraction.AddTwoHandedItem` Interactor self "None"))
    (if _success_
      (set `self.InUse?` true))))

(event `E_DropTwoHandedItem`
  (params (`SumulatePhysics?` :type Boolean))
  (set `self.InUse?` false)
  (`PrimitiveComponent.SetSimulatePhysics` (`self.PickupMesh`) `SumulatePhysics?`))

(fn `GetItemInfo`
  (returns (ItemInfo :type "/Game/LMiTW/Blueprints/Structures/S_ItemInfo Structure"))
  (return (`self.ItemInfo`)))

(fn `UserConstructionScript`
  (`StaticMeshComponent.SetStaticMesh` (`self.PickupMesh`) (`.StaticMesh_23_9F5223F84DD7D2895F9C5585A125810E` (break `/Game/LMiTW/Blueprints/Structures/S_ItemInfo` (`self.ItemInfo`)))))