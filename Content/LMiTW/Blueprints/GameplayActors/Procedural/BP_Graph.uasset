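; Procedural level actor that, when Work is set, builds a graph of node actors linked by shared doors at BeginPlay.
; It assigns node IDs, has switchers register with doors, then records unique door edges and a flattened boolean adjacency matrix.
; A path search between hardcoded start and target IDs yields an 888-delimited array, which a game-design filter narrows to FilteredPath.
; Edges, matrix and paths are logged to GraphText.txt before FinishWork is set.
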(event `self.ReceiveBeginPlay`
  (if (`self.work?`)
    (`|ExecutionSequence`
      (:`then_0`
        ;[1 0.01374 0] c
        (`self.SetIdToNodes`)
        (bind _outactors (`GameplayStatics.GetAllActorsOfClass` (`self.NodeClass`)))
        (bind _returnvalue (`KismetArrayLibrary.Array_Length` _outactors))
        (set `self.adjacecnyMatrixSize` (* _returnvalue _returnvalue))
        ;[1 1 1] Add references-switchers to Doors
        (bind _outactors_2 (`GameplayStatics.GetAllActorsOfClass` "/Game/LMiTW/Blueprints/GameplayActors/Switcher/BP_MasterSwitcher.BP_MasterSwitcher_C"))
        (for _array_element _outactors_2
          (`/Game/LMiTW/Blueprints/GameplayActors/Switcher/BP_MasterSwitcher.Event_AddSwitcherToDoorBP` _array_element)))
      (:`then_1`
        (`KismetArrayLibrary.Array_Clear` (`self.edges`))
        (`KismetArrayLibrary.Array_Clear` (`self.Graph2dMatrix`))
        ;[1 1 1] Add elements for 2d matrix
        (for _ (range (`self.adjacecnyMatrixSize`))
          (`KismetArrayLibrary.Array_Add` (`self.Graph2dMatrix`))))
      (:`then_2`
        ;[1 1 1] Node
        (bind _outactors_3 (`GameplayStatics.GetAllActorsOfClass` (`self.NodeClass`)))
        (for (_array_element_2 _array_index) _outactors_3
          (for _array_element_3 (`/Game/LMiTW/Blueprints/GameplayActors/Procedural/BP_Node.BPDoors` _array_element_2)
            (for (_array_element_4 _array_index_2) _outactors_3 :!label _label
              (if (!= _array_index_2 _array_index)
                (for _array_element_5 (`/Game/LMiTW/Blueprints/GameplayActors/Procedural/BP_Node.BPDoors` _array_element_4)
                  (if (== _array_element_5 _array_element_3)
                    (bind _isitnewelement_ (`self.CompareValidDoor` _array_element_3))
                    (if _isitnewelement_
                      (`self.AddElementToEdgeMatrix` _array_element_2 _array_element_4 _array_element_3)
                      (bind _id (`/Game/LMiTW/Blueprints/GameplayActors/Procedural/BP_Node.id` _array_element_2))
                      (bind _id_2 (`/Game/LMiTW/Blueprints/GameplayActors/Procedural/BP_Node.id` _array_element_4))
                      ;[1 1 1] Поменять имя на более понятное
                      (bind _arrout (`self.setNewNodeConnectToMatrix` (`self.Graph2dMatrix`) _id _id_2))
                      (set `self.Graph2dMatrix` _arrout)
                      ;[1 1 1] Set Node TextName
                      (`/Game/LMiTW/Blueprints/GameplayActors/Procedural/BP_Node.SetNewIndexInName` _array_element_2 _id)
                      (`/Game/LMiTW/Blueprints/GameplayActors/Procedural/BP_Node.SetNewIndexInName` _array_element_4 _id_2)
                      (`|ExecutionSequence`
                        (:`then_0`
                          (break))
                        (:`then_1`
                          (goto _label :!via `Break`))))))))))
        (`KismetSystemLibrary.Delay` 0.0)
        (bind (_arrpathes888 _returnvalue_2) (`self.pathesSearcher` (`self.Graph2dMatrix`) 0 7))
        (if _returnvalue_2
          (bind _output_get (set `self.PathesID` _arrpathes888))
          (bind _filteredpath (`self.pathesGameDesignFilter` _output_get (`self.PathFilterType`) (`self.InAmountOfRooms`) (`self.In Length Percent`)))
          (set `self.FilteredPath` _filteredpath)
          (`self.LogToFile`)
          (set `self.FinishWork?` true))))))

(fn `AddElementToAdjacencyMatrix`
  (params (Node1ArrIndex :type Integer) (Node2ArrIndex :type Integer) (Node1 :type "/Game/LMiTW/Blueprints/GameplayActors/Procedural/BP_Node Object Reference") (Node2 :type "/Game/LMiTW/Blueprints/GameplayActors/Procedural/BP_Node Object Reference"))
  (locals (Node1Local :type "/Game/LMiTW/Blueprints/GameplayActors/Procedural/BP_Node Object Reference") (Node2Local :type "/Game/LMiTW/Blueprints/GameplayActors/Procedural/BP_Node Object Reference"))
  (bind _bpnodeout (`self.AddElementWithCheckout` Node1))
  (bind _bpnodeout_2 (`self.AddElementWithCheckout` Node2))
  (bind _outactors (`GameplayStatics.GetAllActorsOfClass` (`self.NodeClass`)))
  (`KismetArrayLibrary.Array_Set` _outactors Node1ArrIndex _bpnodeout)
  (`KismetArrayLibrary.Array_Set` _outactors Node2ArrIndex _bpnodeout_2)
  (return))

(fn `AddElementToEdgeMatrix`
  (params (vertex1 :type "/Game/LMiTW/Blueprints/GameplayActors/Procedural/BP_Node Object Reference") (vertex2 :type "/Game/LMiTW/Blueprints/GameplayActors/Procedural/BP_Node Object Reference") (door :type "/Game/LMiTW/Blueprints/GameplayActors/Door/BP_DoorSlider Object Reference") (controlPanel :type "/Game/LMiTW/Blueprints/GameplayActors/Switcher/BP_DoorControlPanel Object Reference"))
  (bind _returnvalue (`KismetArrayLibrary.Array_Length` (`self.edges`)))
  (`KismetArrayLibrary.Array_Add` (`self.edges`) (make `/Game/LMiTW/Blueprints/Structures/S_GraphEdgeInfo` _returnvalue vertex1 vertex2 door controlPanel))
  ;[1 1 1] Log to Display
  (if (== _returnvalue 8)
    (for _array_element (`self.edges`)
      (bind (_number _vertex1 _vertex2 _door) (break `/Game/LMiTW/Blueprints/Structures/S_GraphEdgeInfo` _array_element))
      (`KismetSystemLibrary.PrintString` (`KismetStringLibrary.Conv_IntToString` _number) false false)
      (`KismetSystemLibrary.PrintString` (`KismetStringLibrary.Concat_StrStr` (`KismetSystemLibrary.GetDisplayName` _vertex1) " ------- (" (`KismetSystemLibrary.GetDisplayName` _door) ") ------> " (`KismetSystemLibrary.GetDisplayName` _vertex2)) false false (struct :`G` 0.66 :`B` 1.0 :`A` 1.0) 30.0))))

(fn `AddElementWithCheckout`
  (params (BPNodeIn :type "/Game/LMiTW/Blueprints/GameplayActors/Procedural/BP_Node Object Reference"))
  (returns (BPNodeOut :type "/Game/LMiTW/Blueprints/GameplayActors/Procedural/BP_Node Object Reference"))
  ;[1 1 1] In Matrix already?
  (if (<= (`/Game/LMiTW/Blueprints/GameplayActors/Procedural/BP_Node.id` BPNodeIn) (- (`KismetArrayLibrary.Array_Length` (`self.adjacencyMatrix`)) 1))
    ;[0.872 0 1] False Return
    (return BPNodeIn)))

(fn `CompareValidDoor`
  (params (doorToCompare :type "/Game/LMiTW/Blueprints/GameplayActors/Door/BP_DoorSlider Object Reference"))
  (returns (`IsItNewElement?` :type Boolean))
  (locals (`GraphAlreadyHaveThisEdge?` :type Boolean))
  (for _array_element (`self.edges`)
    (if (== (`.door_15_785CF301473C49D04B2048B6696F4B73` (break `/Game/LMiTW/Blueprints/Structures/S_GraphEdgeInfo` _array_element)) doorToCompare)
      (set `local.GraphAlreadyHaveThisEdge?` true)))
  (return (not (`local.GraphAlreadyHaveThisEdge?`))))

(fn `LogToFile`
  (returns (`Success?` :type Boolean))
  (locals (StringBuffer :type String) (counter :type Integer))
  (bind _returnvalue (`KismetMathLibrary.FTrunc` (`KismetMathLibrary.Sqrt` (`KismetMathLibrary.Conv_IntToDouble` (`self.adjacecnyMatrixSize`)))))
  (bind _returnvalue_2 (- _returnvalue 1))
  (`|ExecutionSequence`
    (:`then_0`
      (`GeneratorFunctionLibrary.customSaveStringToFile` "===LOG START===" "GraphText.txt")
      ;[1 1 1] log branches
      (for _array_element (`self.edges`)
        (bind (_number _vertex1 _vertex2 _door) (break `/Game/LMiTW/Blueprints/Structures/S_GraphEdgeInfo` _array_element))
        (bind _returnvalue_3 (`KismetStringLibrary.Concat_StrStr` (`KismetSystemLibrary.GetDisplayName` _vertex1) " ------- (" (`KismetSystemLibrary.GetDisplayName` _door) ") ------> " (`KismetSystemLibrary.GetDisplayName` _vertex2)))
        (`GeneratorFunctionLibrary.customSaveStringToFile` _returnvalue_3 "GraphText.txt")
        (`KismetSystemLibrary.PrintString` _returnvalue_3 false false (struct :`R` 1.0 :`G` 0.004949 :`B` 0.174957 :`A` 1.0) 180.0))
      (`GeneratorFunctionLibrary.customSaveStringToFile` "" "GraphText.txt"))
    (:`then_1`
      ;[1 1 1] Log 2d Matrix
      (bind _output_get (set `local.StringBuffer` "Edges properties:"))
      (`GeneratorFunctionLibrary.customSaveStringToFile` _output_get "GraphText.txt")
      (set `local.StringBuffer` "")
      (for _index (range (+ _returnvalue_2 1))
        (set `local.StringBuffer` "")
        (for _index_2 (range (+ _returnvalue_2 1))
          (bind _returnvalue_4 (+ _index_2 (* _index _returnvalue)))
          (set `local.StringBuffer` (`KismetStringLibrary.Concat_StrStr` (`local.StringBuffer`) (`KismetStringLibrary.Conv_IntToString` (`KismetMathLibrary.SelectInt` 1 0 (`|GetArrayItem` (`self.Graph2dMatrix`) _returnvalue_4))) "  "))
          (`KismetSystemLibrary.PrintString` (`KismetStringLibrary.Conv_IntToString` _returnvalue_4) false false (struct :`R` 1.0 :`G` 0.905104 :`B` 0.310215 :`A` 1.0) 4.0))
        (`GeneratorFunctionLibrary.customSaveStringToFile` (`local.StringBuffer`) "GraphText.txt"))
      (`GeneratorFunctionLibrary.customSaveStringToFile` "" "GraphText.txt"))
    (:`then_2`
      (`|ExecutionSequence`
        (:`then_0`
          ;[1 1 1] Log all pathes
          (bind _output_get_2 (set `local.StringBuffer` "Generated Pathes:"))
          (`GeneratorFunctionLibrary.customSaveStringToFile` _output_get_2 "GraphText.txt")
          (set `local.StringBuffer` (`KismetStringLibrary.Concat_StrStr` "[" "0" "]  "))
          (for _array_element_2 (`self.PathesID`)
            (if (!= _array_element_2 888)
              (set `local.StringBuffer` (`KismetStringLibrary.Concat_StrStr` (`local.StringBuffer`) (`KismetStringLibrary.Conv_IntToString` _array_element_2) "  "))
              (else
                (`GeneratorFunctionLibrary.customSaveStringToFile` (`local.StringBuffer`) "GraphText.txt")
                (bind _result (`/Engine/EditorBlueprintResources/StandardMacros.IncrementInt` (`local.counter`))
                  (:`  `
                    (set `local.StringBuffer` (`KismetStringLibrary.Concat_StrStr` "[" (`KismetStringLibrary.Conv_IntToString` _result) "]  "))))))))
        (:`then_1`
          ;[1 1 1] Filtered Path
          (set `local.StringBuffer` "")
          (for _array_element_3 (`self.FilteredPath`)
            (set `local.StringBuffer` (`KismetStringLibrary.Concat_StrStr` (`local.StringBuffer`) (`KismetStringLibrary.Conv_IntToString` _array_element_3) "  ")))
          (`GeneratorFunctionLibrary.customSaveStringToFile` "Filtered Path:" "GraphText.txt")
          (`GeneratorFunctionLibrary.customSaveStringToFile` (`local.StringBuffer`) "GraphText.txt"))
        (:`then_2`
          ;[1 1 1] Log end
          (`GeneratorFunctionLibrary.customSaveStringToFile` "===LOG END===" "GraphText.txt")
          (`GeneratorFunctionLibrary.customSaveStringToFile` "" "GraphText.txt")
          (`GeneratorFunctionLibrary.customSaveStringToFile` "" "GraphText.txt")
          (`GeneratorFunctionLibrary.customSaveStringToFile` "" "GraphText.txt")
          (return true))))))

(fn `SetIdToDoors`
  (bind _outactors (`GameplayStatics.GetAllActorsOfClass` (`self.DoorClass`)))
  (for (_array_element _array_index) _outactors
    (set `/Game/LMiTW/Blueprints/GameplayActors/Door/BP_MasterDoor.Id` _array_index _array_element)))

(fn `SetIdToNodes`
  (bind _outactors (`GameplayStatics.GetAllActorsOfClass` (`self.NodeClass`)))
  (for (_array_element _array_index) _outactors
    (set `/Game/LMiTW/Blueprints/GameplayActors/Procedural/BP_Node.id` (+ _array_index 0) _array_element)))

(fn `UserConstructionScript`)