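; BP_Button is an interactable switcher actor that activates when the player interacts with it and displays its pressed state on a widget.
; Interact calls Activate, leaving the switching logic to the parent class.
; Overrides of Init and SetControlledActorState run the parent logic, then refresh the widget text to the pressed or not-pressed message based on IsActivated.
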(event `/Game/LMiTW/Blueprints/Interface/BPI_Interactable.Interact`
  (params (Interactor :type "/Game/LMiTW/Blueprints/Character/BP_LMPlayerCharacter Object Reference"))
  (`self.Activate`))

(fn `Init`
  (`parent.Init`)
  (`self.UpdateWidgetInfo`))

(fn `SetControlledActorState`
  (params (IsActive :type Boolean))
  (`parent.SetControlledActorState` IsActive)
  (set `self.IsActivated` IsActive)
  (`self.UpdateWidgetInfo`))

(fn `UpdateWidgetInfo`
  (message `/Game/LMiTW/Blueprints/Interface/BPI_SwitcherWidgetInterface.SetWidgetText` (`WidgetComponent.GetWidget` (`self.Widget`)) (select `bool` (`self.IsActivated`) :`false` (`self.NotPressedText`) :`true` (`self.PressedText`))))

(fn `UserConstructionScript`
  (`parent.UserConstructionScript`))