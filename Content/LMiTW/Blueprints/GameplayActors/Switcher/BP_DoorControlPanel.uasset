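; Wall-panel switcher that controls a linked BP_MasterDoor according to a door status and shows its state on a 3D widget.
; SetStatus, applied on BeginPlay, maps each status to an access level and configures the door's mode, enablement and automatic opening; pin-code statuses only set the level.
; When online, Interact activates the door for Unlocked, or for access-level statuses after CheckAccessLevel passes.
; Controlled-actor state changes refresh the widget.
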(event `self.ReceiveBeginPlay`
  (`self.Init`)
  (`self.SetStatus` (`self.Status`)))

(event `/Game/LMiTW/Blueprints/Interface/BPI_Interactable.Interact`
  (params (Interactor :type "/Game/LMiTW/Blueprints/Character/BP_LMPlayerCharacter Object Reference"))
  (if (`self.IsOnline`)
    (switch `/Game/LMiTW/Blueprints/Enums/E_SwitcherStatusRange` (`self.Status`)
      (:`NewEnumerator11`
        ;[1 1 1] Unlocked
        (`self.TryActivateRemoteActor`))
      (:`NewEnumerator1`
        ;[1 1 1] Access level
        (bind _haveaccess (`self.CheckAccessLevel` Interactor :!label _label))
        (if _haveaccess
          (`self.TryActivateRemoteActor`)
          (else
            (`KismetSystemLibrary.PrintString` "PDA Have no access"))))
      (:`NewEnumerator2`
        (goto _label))
      (:`NewEnumerator3`
        (goto _label))
      (:`NewEnumerator5`)
      (:`NewEnumerator7`)
      (:`NewEnumerator9`))))

(fn `GetInteractInfo`
  (returns (Info :type "/Game/LMiTW/Blueprints/Structures/S_InteractionInfo Structure"))
  (return (`self.InteractInfo`)))

(fn `GetStatus`
  (returns (outStatus :type "/Game/LMiTW/Blueprints/Enums/E_SwitcherStatusRange Enum"))
  (return (`self.Status`)))

(fn `Init`
  (`parent.Init`)
  (bind _returnvalue (`|CreateWidget` (`self.WidgetClass`)))
  (bind _output_get (set `self.Widget` _returnvalue))
  (`WidgetComponent.SetWidget` (`self.3dWidget`) _output_get)
  (`self.UpdateWidgetInfo`))

(fn `SetAccessLevel`
  (params (InAccessLevel :type "/Game/LMiTW/Blueprints/Enums/E_AcessLevels Enum" :default "NewEnumerator3"))
  (set `self.AccessLevel` InAccessLevel))

(fn `SetControlledActorState`
  (params (IsActive :type Boolean))
  (`parent.SetControlledActorState` IsActive)
  (set `self.IsActivated` IsActive)
  (`self.UpdateWidgetInfo`))

(fn `SetStatus`
  (params (InStatus :type "/Game/LMiTW/Blueprints/Enums/E_SwitcherStatusRange Enum" :default "NewEnumerator0"))
  (bind _output_get (set `self.Status` InStatus))
  (switch `/Game/LMiTW/Blueprints/Enums/E_SwitcherStatusRange` _output_get
    (:`NewEnumerator0`
      ;[1 0 0] Comment
      (bind _asbp_master_door (cast `/Game/LMiTW/Blueprints/GameplayActors/Door/BP_MasterDoor` (`self.ControlledActor`)))
      (`self.SetAccessLevel` "NewEnumerator3")
      (`/Game/LMiTW/Blueprints/GameplayActors/Door/BP_MasterDoor.SetIsEnable` _asbp_master_door false)
      (`/Game/LMiTW/Blueprints/GameplayActors/Door/BP_MasterDoor.SetAutomaticClose` _asbp_master_door true)
      (`/Game/LMiTW/Blueprints/GameplayActors/Door/BP_MasterDoor.SetDisableAutomaticOpen` _asbp_master_door)
      (`/Game/LMiTW/Blueprints/GameplayActors/Door/BP_MasterDoor.E_Close_Door` _asbp_master_door)
      (set `/Game/LMiTW/Blueprints/GameplayActors/Door/BP_MasterDoor.DoorMode` "NewEnumerator1" _asbp_master_door))
    (:`NewEnumerator12`
      ;[1 1 1] Blocked
      (`self.SetAccessLevel` "NewEnumerator3")
      (bind _asbp_master_door_2 (cast `/Game/LMiTW/Blueprints/GameplayActors/Door/BP_MasterDoor` (`self.ControlledActor`)))
      (`/Game/LMiTW/Blueprints/GameplayActors/Door/BP_MasterDoor.SetIsEnable` _asbp_master_door_2 false)
      ;[1 0 0] Comment
      (`/Game/LMiTW/Blueprints/GameplayActors/Door/BP_MasterDoor.E_Close_Door` _asbp_master_door_2)
      (set `/Game/LMiTW/Blueprints/GameplayActors/Door/BP_MasterDoor.DoorMode` "NewEnumerator1" _asbp_master_door_2))
    (:`NewEnumerator13`
      ;[1 1 1] Bypassed
      (`self.SetAccessLevel` "NewEnumerator3")
      (bind _asbp_master_door_3 (cast `/Game/LMiTW/Blueprints/GameplayActors/Door/BP_MasterDoor` (`self.ControlledActor`)))
      ;;[1 0.08657 0] Comment
      (`/Game/LMiTW/Blueprints/GameplayActors/Door/BP_MasterDoor.E_Close_Door` _asbp_master_door_3)
      (message `/Game/LMiTW/Blueprints/Interface/BPI_Interactable.Interact` _asbp_master_door_3 null)
      (`/Game/LMiTW/Blueprints/GameplayActors/Door/BP_MasterDoor.SetAutomaticClose` _asbp_master_door_3 false)
      (`/Game/LMiTW/Blueprints/GameplayActors/Door/BP_MasterDoor.SetIsEnable` _asbp_master_door_3 false)
      ;[1 0 0] Comment
      (set `/Game/LMiTW/Blueprints/GameplayActors/Door/BP_MasterDoor.DoorMode` "NewEnumerator0" _asbp_master_door_3))
    (:`NewEnumerator16`
      ;[1 1 1] Automatic
      (`self.SetAccessLevel` "NewEnumerator3")
      (bind _asbp_master_door_4 (cast `/Game/LMiTW/Blueprints/GameplayActors/Door/BP_MasterDoor` (`self.ControlledActor`)))
      (set `/Game/LMiTW/Blueprints/GameplayActors/Door/BP_MasterDoor.DoorMode` "NewEnumerator0" _asbp_master_door_4)
      (`/Game/LMiTW/Blueprints/GameplayActors/Door/BP_MasterDoor.SetEnableAutomaticOpen` _asbp_master_door_4)
      ;;[1 0 0] Comment
      (`/Game/LMiTW/Blueprints/GameplayActors/Door/BP_MasterDoor.SetAutomaticClose` _asbp_master_door_4 true)
      (`/Game/LMiTW/Blueprints/GameplayActors/Door/BP_MasterDoor.E_Close_Door` _asbp_master_door_4))
    (:`NewEnumerator11`
      ;[1 1 1] Unlock
      (`self.SetAccessLevel` "NewEnumerator3")
      (bind _asbp_master_door_5 (cast `/Game/LMiTW/Blueprints/GameplayActors/Door/BP_MasterDoor` (`self.ControlledActor`) :!label _label))
      (`/Game/LMiTW/Blueprints/GameplayActors/Door/BP_MasterDoor.SetDisableAutomaticOpen` _asbp_master_door_5)
      ;[1 0 0.0781] Comment
      (`/Game/LMiTW/Blueprints/GameplayActors/Door/BP_MasterDoor.SetIsEnable` _asbp_master_door_5 true)
      (`/Game/LMiTW/Blueprints/GameplayActors/Door/BP_MasterDoor.E_Close_Door` _asbp_master_door_5)
      (set `/Game/LMiTW/Blueprints/GameplayActors/Door/BP_MasterDoor.DoorMode` "NewEnumerator1" _asbp_master_door_5))
    (:`NewEnumerator1`
      ;[1 1 1] Access levels
      (`self.SetAccessLevel` "NewEnumerator0")
      (goto _label))
    (:`NewEnumerator2`
      (`self.SetAccessLevel` "NewEnumerator1")
      (goto _label))
    (:`NewEnumerator3`
      (`self.SetAccessLevel` "NewEnumerator2")
      (goto _label))
    (:`NewEnumerator5`
      ;[1 1 1] PinCode
      (`self.SetAccessLevel` "NewEnumerator3" :!label _label_2))
    (:`NewEnumerator7`
      (goto _label_2))
    (:`NewEnumerator9`
      (goto _label_2))))

(fn `UpdateWidgetInfo`
  (`/Game/LMiTW/HUD/GameplayActors/Interactable/WBP_DoorControlPanel.UpdateInfo` (`self.Widget`) (make `/Game/LMiTW/Blueprints/Structures/S_DoorPanelInfo` (`self.IsOnline`) (`self.AccessLevel`) (`self.IsActivated`))))

(fn `UserConstructionScript`
  (`parent.UserConstructionScript`))