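; BP_MasterSwitcher is an interactable switch actor, apparently a base for switchers, that turns a linked ControlledActor on and off.
; Interact calls Activate, which flips IsActivated and calls ActivateControlledActor or DeactivateControlledActor on that actor to match.
; StartFocus and StopFocus toggle custom depth rendering on SwitcherMesh, and GetInteractInfo returns the stored InteractInfo.
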(event `/Game/LMiTW/Blueprints/Interface/BPI_Interactable.Interact`
  (params (Interactor :type "/Game/LMiTW/Blueprints/Character/BP_LMPlayerCharacter Object Reference"))
  ;[1 1 1] Interaction
  (`self.Activate`))

(event `/Game/LMiTW/Blueprints/Interface/BPI_Interactable.StartFocus`
  (`self.SetRenderCustomDepth` true))

(event `/Game/LMiTW/Blueprints/Interface/BPI_Interactable.StopFocus`
  (`self.SetRenderCustomDepth` false))

(fn `Activate`
  (set `self.IsActivated` (not (`self.IsActivated`)))
  (if (`self.IsActivated`)
    (`/Game/LMiTW/Blueprints/Interface/BPI_IndirectAccess.ActivateControlledActor` (`self.ControlledActor`))
    (else
      (`/Game/LMiTW/Blueprints/Interface/BPI_IndirectAccess.DeactivateControlledActor` (`self.ControlledActor`)))))

(fn `GetInteractInfo`
  (returns (Info :type "/Game/LMiTW/Blueprints/Structures/S_InteractionInfo Structure"))
  (return (`self.InteractInfo`)))

(fn `SetRenderCustomDepth`
  (params (Render :type Boolean))
  (`PrimitiveComponent.SetRenderCustomDepth` (`self.SwitcherMesh`) Render))

(fn `UserConstructionScript`)