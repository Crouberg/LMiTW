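; Optimization Blueprint that pushes its performance and quality variables to the engine on BeginPlay.
; A sequence builds console commands for screen percentage, view distance, anti-aliasing, FPS cap, detail mode and scalability groups, plus optional unlit view.
; View distance quality also goes through GameUserSettings, and MotionBlurQuality drives the whole post-process group.
; Command names and values are appended without a separating space.
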(event `self.ReceiveBeginPlay`
  (`|ExecutionSequence`
    (:`then_0`
      (if (`self.UnlitMode?`)
        (`KismetSystemLibrary.ExecuteConsoleCommand` "viewmode unlit" null)))
    (:`then_1`
      ;[1 1 1] 0 to 100
      (`KismetSystemLibrary.ExecuteConsoleCommand` (`KismetStringLibrary.Concat_StrStr` "r.ScreenPercentage " (`KismetStringLibrary.Conv_IntToString` (`self.ScreenPercentage`))) null))
    (:`then_2`
      ;[1 1 1] 0 to 1
      (`KismetSystemLibrary.ExecuteConsoleCommand` (`KismetStringLibrary.Concat_StrStr` "r.ViewDistanceScale " (`KismetStringLibrary.Conv_DoubleToString` (`self.ViewDistanceScale??`))) null))
    (:`then_3`
      (`|ExecutionSequence`
        (:`then_0`
          ;[1 1 1] View distance scale: 0 to 1
          (bind _returnvalue (`GameUserSettings.GetGameUserSettings`))
          (`GameUserSettings.SetViewDistanceQuality` _returnvalue (`self.ViewDistanceQuality`)))
        (:`then_1`
          ;[1 1 1] PostProcess Anti-aliasing: 0 to 1
          (`KismetSystemLibrary.ExecuteConsoleCommand` (`KismetStringLibrary.Concat_StrStr` "r.PostProcessAAQuality " (`KismetStringLibrary.Conv_DoubleToString` (`self.PostProcessAnti-aliasing`))) null))
        (:`then_2`
          ;[1 1 1] Max fps
          (`KismetSystemLibrary.ExecuteConsoleCommand` (`KismetStringLibrary.Concat_StrStr` "t.MaxFPS " (`KismetStringLibrary.Conv_IntToString` (`self.MaxFPS`))) null))
        (:`then_3`
          (`|ExecutionSequence`
            (:`then_0`
              ;[1 1 1] Motion blur quality 0 3
              (`KismetSystemLibrary.ExecuteConsoleCommand` (`KismetStringLibrary.Concat_StrStr` "sg.PostProcessQuality " (`KismetStringLibrary.Conv_IntToString` (`self.MotionBlurQuality`))) null))
            (:`then_1`
              ;[1 1 1] Shadow quality 0 3
              (`KismetSystemLibrary.ExecuteConsoleCommand` (`KismetStringLibrary.Concat_StrStr` "sg.ShadowQuality " (`KismetStringLibrary.Conv_IntToString` (`self.ShadowQuality`))) null))
            (:`then_2`
              ;[1 1 1] Texture quality 0 3
              (`KismetSystemLibrary.ExecuteConsoleCommand` (`KismetStringLibrary.Concat_StrStr` "sg.TextureQuality " (`KismetStringLibrary.Conv_IntToString` (`self.TextureQuality`))) null))
            (:`then_3`
              (`|ExecutionSequence`
                (:`then_0`
                  ;[1 1 1] EffectsQuality 0 3
                  (`KismetSystemLibrary.ExecuteConsoleCommand` (`KismetStringLibrary.Concat_StrStr` "sg.EffectsQuality " (`KismetStringLibrary.Conv_IntToString` (`self.EffectsQuality`))) null))
                (:`then_1`
                  ;[1 1 1] DetailQuality 0 2
                  (`KismetSystemLibrary.ExecuteConsoleCommand` (`KismetStringLibrary.Concat_StrStr` "r.DetailMode " (`KismetStringLibrary.Conv_IntToString` (`self.DetailQuality`))) null))))))))))

(fn `UserConstructionScript`)